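; Debug component that visualizes a character's movement and animation layering.
; It draws arrows for velocity, movement input and target rotation, plus an aim cone and capsule.
; Dynamic material instances on each body-part slot are tinted by lerping layer colors with animation curve values, including hand IK.
; A reset restores either a solid color or a skin and clothing scheme chosen by shirt, pants, shoes and gloves settings.
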(event EventBeginPlay)

(event EventTick
  (params (DeltaSeconds :type Float%20%28single-precision%29)))

(event EventDrawDebugSpheres
  (CallFunction|OnDrawDebugSpheres))

(event EventUpdateColoringSystem
  (CallFunction|OnUpdateColoringSystem))

(event EventSetDynamicMaterials
  (CallFunction|OnSetDynamicMaterials))

(event EventSetResetColors
  (CallFunction|OnSetResetColors))

(fn OnDrawDebugSpheres
  (bind _ownercharacter (Variables|Default|GetOwnerCharacter))
  (bind _ownercharacter_2 (Variables|Default|GetOwnerCharacter))
  (bind _ownercharacter_3 (Variables|Default|GetOwnerCharacter))
  (bind _ownercharacter_4 (Variables|Default|GetOwnerCharacter))
  (bind _returnvalue (Transformation|GetActorLocation _ownercharacter_2))
  (bind _returnvalue_2 (Transformation|GetActorLocation _ownercharacter))
  (bind _returnvalue_3 (Transformation|GetActorLocation _ownercharacter_4))
  (bind _returnvalue_4 (Transformation|GetVelocity _ownercharacter_4))
  (bind _capsulecomponent (Variables|/Script/Engine.Character|GetCapsuleComponent _ownercharacter))
  (bind _capsulecomponent_2 (Variables|/Script/Engine.Character|GetCapsuleComponent _ownercharacter_2))
  (bind _charactermovement (Variables|/Script/Engine.Character|GetCharacterMovement _ownercharacter))
  (bind _capsulecomponent_3 (Variables|/Script/Engine.Character|GetCapsuleComponent _ownercharacter_3))
  (bind _capsulecomponent_4 (Variables|/Script/Engine.Character|GetCapsuleComponent _ownercharacter_4))
  (bind _returnvalue_5 (Components|Capsule|GetScaledCapsuleHalfHeight _capsulecomponent_2))
  (bind _returnvalue_6 (Components|Capsule|GetScaledCapsuleHalfHeight _capsulecomponent))
  (bind _returnvalue_7 (Components|Capsule|GetScaledCapsuleHalfHeight _capsulecomponent_4))
  (bind _returnvalue_8 (Math|Vector|Equal(Vector) _returnvalue_4 "0, 0, 0" 0.0001))
  (bind _returnvalue_9 (Pawn|Components|CharacterMovement|GetCurrentAcceleration _charactermovement))
  (bind _returnvalue_10 (- _returnvalue_5 7.0))
  (bind _returnvalue_11 (- _returnvalue_6 3.5))
  (bind _returnvalue_12 (Math|Vector|Equal(Vector) _returnvalue_9 "0, 0, 0" 0.0001))
  (bind _returnvalue_13 (- _returnvalue_3 (Math|Vector|MakeVector 0.0 0.0 _returnvalue_7)))
  (bind _returnvalue_14 (- _returnvalue (Math|Vector|MakeVector 0.0 0.0 _returnvalue_10)))
  (bind _returnvalue_15 (- _returnvalue_2 (Math|Vector|MakeVector 0.0 0.0 _returnvalue_11)))
  ;[1 1 1] Velocity Arrow
  (Rendering|Debug|DrawDebugArrow _returnvalue_13 (+ _returnvalue_13 (* (Class|KismetMathLibrary|VectorNormalUnsafe (Math|Vector|SelectVector (Math|Rotator|GetRotationXVector (Variables|/Script/CyShooter.ALSBaseCharacter|GetLastVelocityRotation _ownercharacter_4)) _returnvalue_4 _returnvalue_8)) (Math|Float|MapRangeClamped (Math|Vector|VectorLength _returnvalue_4) 0.0 (Variables|/Script/Engine.CharacterMovementComponent|GetMaxWalkSpeed (Variables|/Script/Engine.Character|GetCharacterMovement _ownercharacter_4)) 5e+01 75.0))) 6e+01 (Math|Color|SelectColor "(R=0.250000,G=0.000000,B=0.250000,A=1.000000)" "(R=1.000000,G=0.000000,B=1.000000,A=1.000000)" _returnvalue_8) 0.0 5.0)
  ;[1 1 1] Movement Input Arrow
  (Rendering|Debug|DrawDebugArrow _returnvalue_15 (+ _returnvalue_15 (* (Class|KismetMathLibrary|VectorNormalUnsafe (Math|Vector|SelectVector (Math|Rotator|GetRotationXVector (Variables|/Script/CyShooter.ALSBaseCharacter|GetLastMovementInputRotation _ownercharacter)) _returnvalue_9 _returnvalue_12)) (Math|Float|MapRangeClamped (/ (Math|Vector|VectorLength _returnvalue_9) (Class|CharacterMovementComponent|GetMaxAcceleration _charactermovement)) 0.0 1.0 5e+01 75.0))) 5e+01 (Math|Color|SelectColor "(R=0.250000,G=0.125000,B=0.000000,A=1.000000)" "(R=1.000000,G=0.500000,B=0.000000,A=1.000000)" _returnvalue_12) 0.0 3.0)
  ;[1 1 1] Target Rotation Arrow
  (Rendering|Debug|DrawDebugArrow _returnvalue_14 (+ _returnvalue_14 (* (Class|KismetMathLibrary|VectorNormalUnsafe (Math|Rotator|GetRotationXVector (Variables|/Script/CyShooter.ALSBaseCharacter|GetTargetRotation _ownercharacter_2))) 5e+01)) 5e+01 "(R=0.000000,G=0.333333,B=1.000000,A=1.000000)" 0.0 3.0)
  ;[1 1 1] Aiming Rotation Cone
  (Class|KismetSystemLibrary|DrawDebugConeinDegrees (Transformation|GetSocketLocation (Variables|/Script/Engine.Character|GetMesh (Variables|Default|GetOwnerCharacter)) "FP_Camera") (Class|KismetMathLibrary|VectorNormalUnsafe (Math|Rotator|GetRotationXVector (Pawn|GetControlRotation (Variables|Default|GetOwnerCharacter) :!class /Script/Engine.Pawn))) 1e+02 3e+01 3e+01 8 "(R=0.000000,G=0.500000,B=1.000000,A=1.000000)" 0.0 0.5)
  ;[1 1 1] Capsule
  (Rendering|Debug|DrawDebugCapsule (Transformation|GetActorLocation _ownercharacter_3) (Components|Capsule|GetScaledCapsuleHalfHeight _capsulecomponent_3) (Components|Capsule|GetScaledCapsuleRadius _capsulecomponent_3) (Transformation|GetActorRotation _ownercharacter_3) "(R=0.000000,G=0.000000,B=0.000000,A=1.000000)" 0.0 0.3))

(fn OnUpdateColoringSystem
  (bind _ownercharacter (Variables|Default|GetOwnerCharacter))
  (bind _ownercharacter_2 (Variables|Default|GetOwnerCharacter))
  (bind _ownercharacter_3 (Variables|Default|GetOwnerCharacter))
  (bind _ownercharacter_4 (Variables|Default|GetOwnerCharacter))
  (bind _ownercharacter_5 (Variables|Default|GetOwnerCharacter))
  (bind _ownercharacter_6 (Variables|Default|GetOwnerCharacter))
  (Utilities|FlowControl|Sequence
    (:then_0
      (Rendering|Material|SetVectorParameterValue (Variables|Default|GetHead) "BaseColor" (Math|Color|Lerp(LinearColor) (Variables|Colors|GetBaseLayerColor) (Math|Color|Lerp(LinearColor) (Variables|Colors|GetOverlayLayerColor) (Variables|Colors|GetAdditiveAmount_Color) (Class|ALSBaseCharacter|GetAnimCurveValue _ownercharacter "Layering_Head_Add")) (Class|ALSBaseCharacter|GetAnimCurveValue _ownercharacter "Layering_Head")) :!class /Script/Engine.MaterialInstanceDynamic)
      (Rendering|Material|SetVectorParameterValue (Variables|Default|GetTorso) "BaseColor" (Math|Color|Lerp(LinearColor) (Variables|Colors|GetBaseLayerColor) (Math|Color|Lerp(LinearColor) (Variables|Colors|GetOverlayLayerColor) (Variables|Colors|GetAdditiveAmount_Color) (Class|ALSBaseCharacter|GetAnimCurveValue _ownercharacter_4 "Layering_Spine_Add")) (Class|ALSBaseCharacter|GetAnimCurveValue _ownercharacter_4 "Layering_Spine")) :!class /Script/Engine.MaterialInstanceDynamic))
    (:then_1
      (Rendering|Material|SetVectorParameterValue (Variables|Default|GetPelvis) "BaseColor" (Math|Color|Lerp(LinearColor) (Variables|Colors|GetBaseLayerColor) (Variables|Colors|GetAdditiveAmount_Color) (Class|ALSBaseCharacter|GetAnimCurveValue (Variables|Default|GetOwnerCharacter) "Layering_Pelvis")) :!class /Script/Engine.MaterialInstanceDynamic)
      (Rendering|Material|SetVectorParameterValue (Variables|Default|GetUpperLegs) "BaseColor" (Math|Color|Lerp(LinearColor) (Variables|Colors|GetBaseLayerColor) (Variables|Colors|GetAdditiveAmount_Color) (Class|ALSBaseCharacter|GetAnimCurveValue (Variables|Default|GetOwnerCharacter) "Layering_Legs")) :!class /Script/Engine.MaterialInstanceDynamic))
    (:then_2
      (Rendering|Material|SetVectorParameterValue (Variables|Default|GetShoulder_L) "BaseColor" (Math|Color|Lerp(LinearColor) (Variables|Colors|GetBaseLayerColor) (Math|Color|Lerp(LinearColor) (Variables|Colors|GetOverlayLayerColor) (Variables|Colors|GetAdditiveAmount_Color) (Class|ALSBaseCharacter|GetAnimCurveValue _ownercharacter_2 "Layering_Arm_L_Add")) (Class|ALSBaseCharacter|GetAnimCurveValue _ownercharacter_2 "Layering_Arm_L")) :!class /Script/Engine.MaterialInstanceDynamic)
      (bind _returnvalue (Rendering|Material|GetVectorParameterValue (Variables|Default|GetLowerArm_L) "BaseColor" :!class /Script/Engine.MaterialInstanceDynamic))
      (Rendering|Material|SetVectorParameterValue (Variables|Default|GetHand_L) "BaseColor" (Math|Color|Lerp(LinearColor) (Math|Color|Lerp(LinearColor) :A _returnvalue :Alpha (Class|ALSBaseCharacter|GetAnimCurveValue _ownercharacter_5 "Layering_Hand_L")) (Variables|Colors|GetHandIK_Color) (Class|ALSBaseCharacter|GetAnimCurveValue _ownercharacter_5 "Enable_HandIK_L")) :!class /Script/Engine.MaterialInstanceDynamic))
    (:then_3
      (Rendering|Material|SetVectorParameterValue (Variables|Default|GetShoulder_R) "BaseColor" (Math|Color|Lerp(LinearColor) (Variables|Colors|GetBaseLayerColor) (Math|Color|Lerp(LinearColor) (Variables|Colors|GetOverlayLayerColor) (Variables|Colors|GetAdditiveAmount_Color) (Class|ALSBaseCharacter|GetAnimCurveValue _ownercharacter_3 "Layering_Arm_R_Add")) (Class|ALSBaseCharacter|GetAnimCurveValue _ownercharacter_3 "Layering_Arm_R")) :!class /Script/Engine.MaterialInstanceDynamic)
      (bind _returnvalue_2 (Rendering|Material|GetVectorParameterValue (Variables|Default|GetLowerArm_R) "BaseColor" :!class /Script/Engine.MaterialInstanceDynamic))
      (Rendering|Material|SetVectorParameterValue (Variables|Default|GetHand_R) "BaseColor" (Math|Color|Lerp(LinearColor) (Math|Color|Lerp(LinearColor) :A _returnvalue_2 :Alpha (Class|ALSBaseCharacter|GetAnimCurveValue _ownercharacter_6 "Layering_Hand_R")) (Variables|Colors|GetHandIK_Color) (Class|ALSBaseCharacter|GetAnimCurveValue _ownercharacter_6 "Enable_HandIK_R")) :!class /Script/Engine.MaterialInstanceDynamic))))

(fn OnSetResetColors
  (if (Variables|Colors|GetSolidColor)
    (Rendering|Material|SetVectorParameterValue (Variables|Default|GetHead) "BaseColor" (Variables|Colors|GetDefaultColor) :!class /Script/Engine.MaterialInstanceDynamic)
    (else
      (Utilities|FlowControl|Sequence
        (:then_0
          (Rendering|Material|SetVectorParameterValue (Variables|Default|GetHead) "BaseColor" (Variables|Colors|GetSkinColor) :!class /Script/Engine.MaterialInstanceDynamic))
        (:then_1
          (switch int (Variables|Colors|GetShirtType)
            (:0
              (Rendering|Material|SetVectorParameterValue (Variables|Default|GetShoulder_L) "BaseColor" (Variables|Colors|GetSkinColor) :!class /Script/Engine.MaterialInstanceDynamic))
            (:1
              (Rendering|Material|SetVectorParameterValue (Variables|Default|GetShoulder_L) "BaseColor" (Variables|Colors|GetShirtColor) :!class /Script/Engine.MaterialInstanceDynamic)
              (Rendering|Material|SetVectorParameterValue (Variables|Default|GetUpperArm_L) "BaseColor" (Variables|Colors|GetSkinColor) :!class /Script/Engine.MaterialInstanceDynamic))
            (:2
              (Rendering|Material|SetVectorParameterValue (Variables|Default|GetShoulder_L) "BaseColor" (Variables|Colors|GetShirtColor) :!class /Script/Engine.MaterialInstanceDynamic)
              (Rendering|Material|SetVectorParameterValue (Variables|Default|GetLowerArm_L) "BaseColor" (Variables|Colors|GetSkinColor) :!class /Script/Engine.MaterialInstanceDynamic))
            (:3
              (Rendering|Material|SetVectorParameterValue (Variables|Default|GetShoulder_L) "BaseColor" (Variables|Colors|GetShirtColor) :!class /Script/Engine.MaterialInstanceDynamic))))
        (:then_2
          (switch int (Variables|Colors|GetPantsType)
            (:0
              (Rendering|Material|SetVectorParameterValue (Variables|Default|GetPelvis) "BaseColor" (Variables|Colors|GetPantsColor) :!class /Script/Engine.MaterialInstanceDynamic)
              (Rendering|Material|SetVectorParameterValue (Variables|Default|GetUpperLegs) "BaseColor" (Variables|Colors|GetSkinColor) :!class /Script/Engine.MaterialInstanceDynamic))
            (:1
              (Rendering|Material|SetVectorParameterValue (Variables|Default|GetPelvis) "BaseColor" (Variables|Colors|GetPantsColor) :!class /Script/Engine.MaterialInstanceDynamic)
              (Rendering|Material|SetVectorParameterValue (Variables|Default|GetLowerLegs) "BaseColor" (Variables|Colors|GetSkinColor) :!class /Script/Engine.MaterialInstanceDynamic))
            (:2
              (Rendering|Material|SetVectorParameterValue (Variables|Default|GetPelvis) "BaseColor" (Variables|Colors|GetPantsColor) :!class /Script/Engine.MaterialInstanceDynamic))))
        (:then_3
          (if (Variables|Colors|GetShoes)
            (Rendering|Material|SetVectorParameterValue (Variables|Default|GetFeet) "BaseColor" (Variables|Colors|GetShoesColor) :!class /Script/Engine.MaterialInstanceDynamic)
            (else
              (Rendering|Material|SetVectorParameterValue (Variables|Default|GetFeet) "BaseColor" (Variables|Colors|GetSkinColor) :!class /Script/Engine.MaterialInstanceDynamic))))
        (:then_4
          (if (Variables|Colors|GetGloves)
            (Rendering|Material|SetVectorParameterValue (Variables|Default|GetHand_L) "BaseColor" (Variables|Colors|GetGlovesColor) :!class /Script/Engine.MaterialInstanceDynamic)
            (else
              (Rendering|Material|SetVectorParameterValue (Variables|Default|GetHand_L) "BaseColor" (Variables|Colors|GetSkinColor) :!class /Script/Engine.MaterialInstanceDynamic))))))))

(fn OnSetDynamicMaterials
  (bind _ownercharacter (Variables|Default|GetOwnerCharacter))
  (bind _mesh (Variables|/Script/Engine.Character|GetMesh _ownercharacter))
  (Utilities|IsValid _ownercharacter
    (:Is%20Valid
      (Utilities|FlowControl|Sequence
        (:then_0
          (bind _returnvalue (Rendering|Material|CreateDynamicMaterialInstance _mesh (Rendering|Material|GetMaterialIndex _mesh "Head_MAT") 0 "None" :!class /Script/Engine.PrimitiveComponent))
          (Variables|Default|SetHead _returnvalue)
          (bind _returnvalue_2 (Rendering|Material|CreateDynamicMaterialInstance _mesh (Rendering|Material|GetMaterialIndex _mesh "Torso_MAT") 0 "None" :!class /Script/Engine.PrimitiveComponent))
          (Variables|Default|SetTorso _returnvalue_2)
          (bind _returnvalue_3 (Rendering|Material|CreateDynamicMaterialInstance _mesh (Rendering|Material|GetMaterialIndex _mesh "Pelvis_MAT") 0 "None" :!class /Script/Engine.PrimitiveComponent))
          (Variables|Default|SetPelvis _returnvalue_3))
        (:then_1
          (bind _returnvalue_4 (Rendering|Material|CreateDynamicMaterialInstance _mesh (Rendering|Material|GetMaterialIndex _mesh "UpperLeg_MAT") 0 "None" :!class /Script/Engine.PrimitiveComponent))
          (Variables|Default|SetUpperLegs _returnvalue_4)
          (bind _returnvalue_5 (Rendering|Material|CreateDynamicMaterialInstance _mesh (Rendering|Material|GetMaterialIndex _mesh "LowerLeg_MAT") 0 "None" :!class /Script/Engine.PrimitiveComponent))
          (Variables|Default|SetLowerLegs _returnvalue_5)
          (bind _returnvalue_6 (Rendering|Material|CreateDynamicMaterialInstance _mesh (Rendering|Material|GetMaterialIndex _mesh "Feet_MAT") 0 "None" :!class /Script/Engine.PrimitiveComponent))
          (Variables|Default|SetFeet _returnvalue_6))
        (:then_2
          (bind _returnvalue_7 (Rendering|Material|CreateDynamicMaterialInstance _mesh (Rendering|Material|GetMaterialIndex _mesh "Shoulder_L_MAT") 0 "None" :!class /Script/Engine.PrimitiveComponent))
          (Variables|Default|SetShoulder_L _returnvalue_7)
          (bind _returnvalue_8 (Rendering|Material|CreateDynamicMaterialInstance _mesh (Rendering|Material|GetMaterialIndex _mesh "UpperArm_L_MAT") 0 "None" :!class /Script/Engine.PrimitiveComponent))
          (Variables|Default|SetUpperArm_L _returnvalue_8)
          (bind _returnvalue_9 (Rendering|Material|CreateDynamicMaterialInstance _mesh (Rendering|Material|GetMaterialIndex _mesh "LowerArm_L_MAT") 0 "None" :!class /Script/Engine.PrimitiveComponent))
          (Variables|Default|SetLowerArm_L _returnvalue_9)
          (bind _returnvalue_10 (Rendering|Material|CreateDynamicMaterialInstance _mesh (Rendering|Material|GetMaterialIndex _mesh "Hand_L_MAT") 0 "None" :!class /Script/Engine.PrimitiveComponent))
          (Variables|Default|SetHand_L _returnvalue_10))
        (:then_3
          (bind _returnvalue_11 (Rendering|Material|CreateDynamicMaterialInstance _mesh (Rendering|Material|GetMaterialIndex _mesh "Shoulder_R_MAT") 0 "None" :!class /Script/Engine.PrimitiveComponent))
          (Variables|Default|SetShoulder_R _returnvalue_11)
          (bind _returnvalue_12 (Rendering|Material|CreateDynamicMaterialInstance _mesh (Rendering|Material|GetMaterialIndex _mesh "UpperArm_R_MAT") 0 "None" :!class /Script/Engine.PrimitiveComponent))
          (Variables|Default|SetUpperArm_R _returnvalue_12)
          (bind _returnvalue_13 (Rendering|Material|CreateDynamicMaterialInstance _mesh (Rendering|Material|GetMaterialIndex _mesh "LowerArm_R_MAT") 0 "None" :!class /Script/Engine.PrimitiveComponent))
          (Variables|Default|SetLowerArm_R _returnvalue_13)
          (bind _returnvalue_14 (Rendering|Material|CreateDynamicMaterialInstance _mesh (Rendering|Material|GetMaterialIndex _mesh "Hand_R_MAT") 0 "None" :!class /Script/Engine.PrimitiveComponent))
          (Variables|Default|SetHand_R _returnvalue_14))
        (:then_4
          (return))))))